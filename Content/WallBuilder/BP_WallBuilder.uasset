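; BP_WallBuilder is a construction-script tool that builds a straight row of hotel exterior wall segments.
; It loops over WallSegments, adding local-space instances of one 2M wall mesh to an InstancedStaticMesh component, rotated and spaced along X by the mesh width.
; ChosenMaterial overrides the first material slot.
; An unconnected loop based on a random WallType entry never runs, so every segment uses the same mesh.
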(fn ConstructionScript
  ;[1 1 1] Wall Section Script
  ;;[0.5239 0.92 1] Subtracts -1 from Index for the desired amount of segments
  (for _index (range 0 (- (Variables|Default|GetWall_Segments) 1))
    ;;[0.4947 0.8794 1] Create Segment
    (Components|StaticMesh|SetStaticMesh (Variables|Default|GetInstancedStaticMesh) "/Game/Cold_Case_Assets/Exported_FBXs/Exterior/ExteriorBuildingAssets/Ext_Wall/Hotel_Exterior_Wall_2M.Hotel_Exterior_Wall_2M")
    (Components|InstancedStaticMesh|AddInstance (Variables|Default|GetInstancedStaticMesh) (Math|Transform|MakeTransform (Math|Vector|MakeVector (Math|Conversions|ToFloat(Integer) (* _index 200)) 0.0 0.0) "0.000000,90.000000,0.000000") false)
    (Rendering|Material|SetMaterial (Variables|Default|GetInstancedStaticMesh) 0 (Variables|Default|GetChosenMaterial))))