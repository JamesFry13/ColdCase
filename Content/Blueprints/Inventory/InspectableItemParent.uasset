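; InspectableItemParent is a base Blueprint for inventory items that can be picked up in the world.
; PickupItem prints a debug message, triggers DestroyItem and returns the item's ItemType to the caller.
; DestroyItem removes the actor after a short delay.
; Unconnected leftover logic would create and remove an item prompt widget for the first-person character, but it never runs.
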(event Custom|DestroyItem
  (Utilities|FlowControl|Delay 0.2)
  (Actor|DestroyActor))

(fn ConstructionScript)

(fn PickupItem
  (Development|PrintString "Item picked")
  (CallFunction|DestroyItem)
  (return (Variables|Default|GetItemType)))