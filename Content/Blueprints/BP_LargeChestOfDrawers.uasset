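; Interactive chest of drawers whose drawers the player slides open and shut individually.
; DrawerInteract line-traces from the first-person camera and takes the hit static mesh component as the drawer, with debug drawing left on.
; The drawer's relative Y decides between opening and closing, each playing a sound and a timeline that lerps it along Y.
; CanOpen blocks re-triggering during movement.
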(event EventDrawerInteract
  (bind _returnvalue (Transformation|GetActorLocation))
  ;[0.3708 1 0.3656] Main Functionality
  (if (Variables|Default|GetCanOpen)
    (Variables|Default|SetCanOpen false)
    (bind _asbp_first_person_character (Utilities|Casting|CastToBP_FirstPersonCharacter (Game|GetPlayerCharacter 0)))
    (bind (_outhit _returnvalue_2) (Collision|LineTraceForObjects (Transformation|GetWorldLocation (Variables|/Game/Blueprints/BP_FirstPersonCharacter.BP_FirstPersonCharacter_C|GetFirstPersonCamera _asbp_first_person_character)) (+ (Transformation|GetWorldLocation (Variables|/Game/Blueprints/BP_FirstPersonCharacter.BP_FirstPersonCharacter_C|GetFirstPersonCamera _asbp_first_person_character)) (* (Math|Vector|GetForwardVector (Variables|/Game/Blueprints/BP_FirstPersonCharacter.BP_FirstPersonCharacter_C|GetFirstPersonCamera _asbp_first_person_character)) (Math|Vector|MakeVector 5e+02 5e+02 5e+02))) (Utilities|Array|MakeArray "ObjectTypeQuery2") false 0 "ForDuration" false))
    (if _returnvalue_2
      (bind _asstatic_mesh_component (Utilities|Casting|CastToStaticMeshComponent (.HitComponent (Collision|BreakHitResult _outhit))))
      (Variables|Default|SetMeshREF _asstatic_mesh_component)
      (if (not (>= (.y (Variables|/Script/Engine.SceneComponent|GetRelativeLocation _asstatic_mesh_component)) 45.0))
        (Audio|PlaySoundatLocation "/Game/Sounds/DoorOpen.DoorOpen" _returnvalue "0, 0, 0" 1.0 1.0 0.0 0 0 0 0)
        (Variables|Default|SetStartLoc (Math|Vector|MakeVector (.x (Variables|/Script/Engine.SceneComponent|GetRelativeLocation (Variables|Default|GetMeshREF))) (.y (Variables|/Script/Engine.SceneComponent|GetRelativeLocation (Variables|Default|GetMeshREF))) (.z (Variables|/Script/Engine.SceneComponent|GetRelativeLocation (Variables|Default|GetMeshREF)))))
        (Variables|Default|SetEndLoc (Math|Vector|MakeVector (.x (Variables|/Script/Engine.SceneComponent|GetRelativeLocation (Variables|Default|GetMeshREF))) (+ (.y (Variables|/Script/Engine.SceneComponent|GetRelativeLocation (Variables|Default|GetMeshREF))) 45.0) (.z (Variables|/Script/Engine.SceneComponent|GetRelativeLocation (Variables|Default|GetMeshREF)))))
        (bind _open (Timeline|OpenDrawer PlayFromStart)
          (:Update
            (Transformation|SetRelativeLocation (Variables|Default|GetMeshREF) (Math|Vector|Lerp(Vector) (Variables|Default|GetStartLoc) (Variables|Default|GetEndLoc) _open) false false))
          (:Finished
            (Variables|Default|SetCanOpen true)))
        (else
          (Audio|PlaySoundatLocation "/Engine/VREditor/Sounds/UI/Dockable_Window_Close.Dockable_Window_Close" _returnvalue "0, 0, 0" 1.0 1.0 0.0 0 0 0 0)
          ;[1 0 0] Close
          (Variables|Default|SetStartLoc (Math|Vector|MakeVector (.x (Variables|/Script/Engine.SceneComponent|GetRelativeLocation (Variables|Default|GetMeshREF))) (.y (Variables|/Script/Engine.SceneComponent|GetRelativeLocation (Variables|Default|GetMeshREF))) (.z (Variables|/Script/Engine.SceneComponent|GetRelativeLocation (Variables|Default|GetMeshREF)))))
          (Variables|Default|SetEndLoc (Math|Vector|MakeVector (.x (Variables|/Script/Engine.SceneComponent|GetRelativeLocation (Variables|Default|GetMeshREF))) (- (.y (Variables|/Script/Engine.SceneComponent|GetRelativeLocation (Variables|Default|GetMeshREF))) 45.0) (.z (Variables|/Script/Engine.SceneComponent|GetRelativeLocation (Variables|Default|GetMeshREF)))))
          (bind _open_2 (Timeline|Close PlayFromStart)
            (:Update
              (Transformation|SetRelativeLocation (Variables|Default|GetMeshREF) (Math|Vector|Lerp(Vector) (Variables|Default|GetStartLoc) (Variables|Default|GetEndLoc) _open_2) false false))
            (:Finished
              (Variables|Default|SetCanOpen true)))))
      (else
        (Variables|Default|SetCanOpen true)))))

(event EventBeginPlay
  (Input|EnableInput (Game|GetPlayerController 0) 0))

(fn ConstructionScript)