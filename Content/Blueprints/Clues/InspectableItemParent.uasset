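; Base Blueprint for inspectable clue items that the player can examine and pick up.
; Inspected waits briefly, then shows the ClueInspect_Keycard widget, hard-coded in this parent, and calls AddItemMessage on the player inventory widgets found by class lookup.
; PickupItem prints a debug string, triggers a short delayed self-destroy and returns the item's type, text and clue number to the caller.
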(event Custom|DestroyItem
  (Utilities|FlowControl|Delay 0.2)
  (Actor|DestroyActor))

(event Custom|Inspected
  (Utilities|FlowControl|Delay 1.0)
  (bind _returnvalue (UserInterface|CreateWidget "/Game/Widgets/Clues/ClueInspect_Keycard.ClueInspect_Keycard_C" (Game|GetPlayerController 0)))
  (UserInterface|Viewport|AddtoViewport _returnvalue 0)
  (bind _foundwidgets (Widget|GetAllWidgetsOfClass "/Game/Widgets/Inventory/WBP_PlayerInventory.WBP_PlayerInventory_C" false))
  (Class|BPIAddtoInventory|AddItem(Message) _foundwidgets))

(fn ConstructionScript)

(fn PickupItem
  (Development|PrintString "Item picked")
  (CallFunction|DestroyItem)
  (return (Variables|Default|GetItemType) (Variables|Default|GetItemText) (Variables|Default|GetClueNumber)))