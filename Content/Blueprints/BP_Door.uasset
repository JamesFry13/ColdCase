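; BP_Door is a sliding door that toggles open and closed each time its OpenDoor event fires.
; A FlipFlop alternately plays and reverses a timeline that lerps the door's relative Y position, with a sound for each direction.
; InteractCollider overlaps with BP_FirstPersonCharacter show and remove a WBP_OpenPrompt widget.
; AutoClose is called on timeline updates but is empty, as its delayed-close logic is disconnected.
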(event OnComponentBeginOverlap(InteractCollider)
  (params (OverlappedComponent :type Primitive%20Component%20Object%20Reference) (OtherActor :type Actor%20Object%20Reference) (OtherComp :type Primitive%20Component%20Object%20Reference) (OtherBodyIndex :type Integer) (bFromSweep :type Boolean) (SweepResult :type Hit%20Result%20Structure%20%28by%20ref%29))
  (Utilities|Casting|CastToBP_FirstPersonCharacter OtherActor)
  (bind _returnvalue (UserInterface|CreateWidget "/Game/Widgets/WBP_OpenPrompt.WBP_OpenPrompt_C"))
  (UserInterface|Viewport|AddtoViewport _returnvalue 0))

(event OnComponentEndOverlap(InteractCollider)
  (params (OverlappedComponent :type Primitive%20Component%20Object%20Reference) (OtherActor :type Actor%20Object%20Reference) (OtherComp :type Primitive%20Component%20Object%20Reference) (OtherBodyIndex :type Integer))
  (Utilities|Casting|CastToBP_FirstPersonCharacter OtherActor)
  (Widget|RemovefromParent (stale OnComponentBeginOverlap(InteractCollider) _returnvalue)))

(event Custom|Open%20Door
  (bind _door (Variables|Default|GetDoor))
  (bind _returnvalue (Transformation|GetWorldLocation _door))
  ;[1 1 1] Open/Close Door
  (Utilities|FlowControl|FlipFlop
    (:A
      (Audio|PlaySoundatLocation "/Engine/VREditor/Sounds/UI/Scaling_Up.Scaling_Up" _returnvalue "0, 0, 0" 1.0 1.0 0.0 0 0 0 0)
      (bind _doorfloat (Timeline|Timeline Play)
        (:Update
          (Transformation|SetRelativeLocation (Variables|Default|GetDoor) (Math|Vector|MakeVector 0.0 (Math|Float|Lerp 0.0 115.0 _doorfloat) 0.0) false false)
          (CallFunction|AutoClose))))
    (:B
      (Audio|PlaySoundatLocation "/Engine/VREditor/Sounds/UI/Scaling_Down.Scaling_Down" _returnvalue "0, 0, 0" 1.0 1.0 0.0 0 0 0 0)
      (Timeline|Timeline Reverse))))

(event Custom|AutoClose)

(event EventBeginPlay)

(event Collision|EventActorBeginOverlap
  (params (OtherActor :type Actor%20Object%20Reference)))

(event EventTick
  (params (DeltaSeconds :type Float%20%28single-precision%29)))

(fn ConstructionScript)