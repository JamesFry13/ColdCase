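; Receptionist NPC that shows a talk prompt on overlap and runs a dialogue widget with the player.
; StartDialogue opens WBP_Dialogue with the NPC's Dialogue data, freezing movement, showing the cursor and zooming the first-person character's camera.
; Close, or StartDialogue past the last NPCText line, removes the widget and restores control.
; GoNext and NextDialogue advance the index and clear the text; the construction script positions the Camera from CameraTransform.
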(event OnComponentBeginOverlap(InteractCollider)
  (params (OverlappedComponent :type Primitive%20Component%20Object%20Reference) (OtherActor :type Actor%20Object%20Reference) (OtherComp :type Primitive%20Component%20Object%20Reference) (OtherBodyIndex :type Integer) (bFromSweep :type Boolean) (SweepResult :type Hit%20Result%20Structure%20%28by%20ref%29))
  ;[0 1 0.07825] Interact Prompt
  (bind _returnvalue (UserInterface|CreateWidget "/Game/Widgets/WBP_Talk.WBP_Talk_C"))
  (Input|SetInputModeUIOnly 0 0 "DoNotLock" false)
  (UserInterface|Viewport|AddtoViewport _returnvalue 0))

(event OnComponentEndOverlap(InteractCollider)
  (params (OverlappedComponent :type Primitive%20Component%20Object%20Reference) (OtherActor :type Actor%20Object%20Reference) (OtherComp :type Primitive%20Component%20Object%20Reference) (OtherBodyIndex :type Integer))
  ;[0 1 0.07825] Interact Prompt
  (Widget|RemovefromParent (stale OnComponentBeginOverlap(InteractCollider) _returnvalue)))

(event Custom|close
  (bind _returnvalue (Game|GetPlayerController 0))
  ;[0 0.2242 1] Start Dialogue
  ;;[1 1 1] Remove Dialogue Widget
  (Widget|RemovefromParent (Variables|Default|GetUI))
  (Game|SetGamePaused false)
  (Variables|/Script/Engine.PlayerController|SetbShowMouseCursor _returnvalue false)
  (Pawn|Components|CharacterMovement|SetMovementMode (Variables|/Script/Engine.Character|GetCharacterMovement (Game|GetPlayerCharacter 0)) "MOVE_Walking" 0)
  (Input|SetInputModeGameandUI _returnvalue 0 "DoNotLock" true false)
  (bind _asbp_first_person_character (Utilities|Casting|CastToBP_FirstPersonCharacter (Game|GetPlayerCharacter 0)))
  (Default|CameraZoomOut _asbp_first_person_character))

(event Custom|NextDialogue
  ;[0 0.2242 1] Start Dialogue
  ;;[0 0 0] Progress Dialogue (Deprecated)
  (Math|Integer|IncrementInt (Variables|Default|GetDialogueIndex)
    (:%20%20
      (Variables|/Script/UMG.TextBlock|SetText (Variables|/Game/Widgets/WBP_Dialogue.WBP_Dialogue_C|GetDialogueText (Variables|Default|GetUI)) ""))))

(event EventGoNext
  ;[0 0.2242 1] Start Dialogue
  ;;[0 0 0] Progress Dialogue (Deprecated)
  (Math|Integer|IncrementInt (Variables|Default|GetDialogueIndex)
    (:%20%20
      (Variables|/Script/UMG.TextBlock|SetText (Variables|/Game/Widgets/WBP_Dialogue.WBP_Dialogue_C|GetDialogueText (Variables|Default|GetUI)) ""))))

(event EventBeginPlay)

(event EventStartDialogue
  (bind _returnvalue (Game|GetPlayerController 0))
  (bind _returnvalue_2 (Game|GetPlayerController 0))
  ;[0 0.2242 1] Start Dialogue
  (if (< (Variables|Default|GetDialogueIndex) (Utilities|Array|Length (Variables|Default|GetNPCText)))
    (Variables|Default|GetUI
      (:then)
      (:else
        ;;[1 1 1] Create Dialogue Widget
        (bind _returnvalue_3 (UserInterface|CreateWidget "/Game/Widgets/WBP_Dialogue.WBP_Dialogue_C" _returnvalue (Variables|Default|GetDialogue)))
        (Widget|RemovefromParent (stale OnComponentBeginOverlap(InteractCollider) _returnvalue))
        (bind _output_get (Variables|Default|SetUI _returnvalue_3))
        (UserInterface|Viewport|AddtoViewport _output_get 0)
        (Pawn|Components|CharacterMovement|DisableMovement (Variables|/Script/Engine.Character|GetCharacterMovement (Game|GetPlayerCharacter 0)))
        (Input|SetInputModeUIOnly _returnvalue _returnvalue_3 "DoNotLock" false)
        (Variables|/Script/Engine.PlayerController|SetbShowMouseCursor _returnvalue true)
        (bind _asbp_first_person_character (Utilities|Casting|CastToBP_FirstPersonCharacter (Game|GetPlayerCharacter 0)))
        (Default|CameraZoom _asbp_first_person_character)))
    (else
      ;;[1 1 1] Remove Dialogue Widget
      (Widget|RemovefromParent (Variables|Default|GetUI))
      (Game|SetGamePaused false)
      (Variables|/Script/Engine.PlayerController|SetbShowMouseCursor _returnvalue_2 false)
      (Pawn|Components|CharacterMovement|SetMovementMode (Variables|/Script/Engine.Character|GetCharacterMovement (Game|GetPlayerCharacter 0)) "MOVE_Walking" 0)
      (Input|SetInputModeGameandUI _returnvalue_2 0 "DoNotLock" true false)
      (bind _asbp_first_person_character_2 (Utilities|Casting|CastToBP_FirstPersonCharacter (Game|GetPlayerCharacter 0)))
      (Default|CameraZoomOut _asbp_first_person_character_2))))

(fn ConstructionScript
  (Transformation|SetRelativeTransform (Variables|Components|GetCamera) (Variables|Default|GetCamera%20Transform) false false))