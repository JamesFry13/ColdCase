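; BP_CreditsDoor is a door that, when opened, ends the level and loads the credits level.
; OpenDoor plays keypad and metal door sounds, then runs a timeline that slides the door sideways.
; The timeline's Update pin also drives the camera and audio fade, adds a FadeToBlack widget every update, and opens L_Credits after a delay.
; Locked-door feedback and overlap prompt logic are disconnected leftovers.
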(event OnComponentBeginOverlap(InteractCollider)
  (params (OverlappedComponent :type Primitive%20Component%20Object%20Reference) (OtherActor :type Actor%20Object%20Reference) (OtherComp :type Primitive%20Component%20Object%20Reference) (OtherBodyIndex :type Integer) (bFromSweep :type Boolean) (SweepResult :type Hit%20Result%20Structure%20%28by%20ref%29))
  ;[0 0 0] UI Interaction (Depreceated)
)

(event OnComponentEndOverlap(InteractCollider)
  (params (OverlappedComponent :type Primitive%20Component%20Object%20Reference) (OtherActor :type Actor%20Object%20Reference) (OtherComp :type Primitive%20Component%20Object%20Reference) (OtherBodyIndex :type Integer))
  ;[0 0 0] UI Interaction (Depreceated)
)

(event Custom|Open%20Door
  (bind _door (Variables|Default|GetDoor))
  (bind _returnvalue (Transformation|GetWorldLocation _door))
  ;[0.1146 1 0.216] Open/Close Door
  (Audio|PlaySoundatLocation "/Game/Sounds/UPDATE/ES_Keypad_Door_Lock_1_-_SFX_Producer.ES_Keypad_Door_Lock_1_-_SFX_Producer" _returnvalue "0, 0, 0" 1.2 1.0 0.0 0 0 0 0)
  (Audio|PlaySoundatLocation "/Game/Sounds/UPDATE/ES_Door_Metal_-_SFX_Producer.ES_Door_Metal_-_SFX_Producer" _returnvalue "0, 0, 0" 1.0 1.0 0.0 0 0 0 0)
  (bind _doorfloat (Timeline|Timeline Play)
    (:Update
      (Transformation|SetRelativeLocation (Variables|Default|GetDoor) (Math|Vector|MakeVector 0.0 (Math|Float|Lerp 0.0 115.0 _doorfloat) 0.0) false false)
      (CameraFades|StartCameraFade :self (Game|GetPlayerCameraManager 0) :ToAlpha 1.0 :Duration 2.0 :bShouldFadeAudio true :bHoldWhenFinished true)
      (bind _returnvalue_2 (UserInterface|CreateWidget "/Game/Widgets/FadeToBlack.FadeToBlack_C"))
      (UserInterface|Viewport|AddtoViewport _returnvalue_2 0)
      (Utilities|FlowControl|Delay 3.0)
      (Game|OpenLevel(byObjectReference) "/Game/Levels/L_Credits.L_Credits"))))

(fn ConstructionScript)