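; Exterior door Blueprint that animates open and transitions the player to the Int_Hotel level.
; The OpenExt event plays a door sound and starts a timeline that lerps the ExtDoor's relative rotation.
; The camera fade, delayed loading screen widget and delayed level open are all chained to the timeline's Update output, not Finished.
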(event Custom|OpenExt
  ;[0.1718 1 0.4493] Door Animation/Level Transition
  (Audio|PlaySoundatLocation "/Game/Sounds/DoorOpen.DoorOpen" (Transformation|GetWorldLocation (Variables|Default|GetExtDoor)) "0, 0, 0" 1.0 1.0 0.6 0 0 0 0)
  (bind _doorfloat (Timeline|Timeline PlayFromStart)
    (:Update
      (Transformation|SetRelativeRotation (Variables|Default|GetExtDoor) (Math|Rotator|Lerp(Rotator) "0, 0, 0" "0.000000,12.000000,0.000000" _doorfloat) false false)
      (CameraFades|StartCameraFade :self (Game|GetPlayerCameraManager 0) :ToAlpha 1.0 :Duration 2.0)
      (Utilities|FlowControl|Delay 1.0)
      (bind _returnvalue (UserInterface|CreateWidget "/Game/Widgets/WBP_LoadingScreen.WBP_LoadingScreen_C"))
      (UserInterface|Viewport|AddtoViewport _returnvalue 0)
      (Utilities|FlowControl|Delay 1.5)
      (Game|OpenLevel(byObjectReference) "/Game/Levels/Int_Hotel.Int_Hotel"))))

(event EventBeginPlay)

(event Collision|EventActorBeginOverlap
  (params (OtherActor :type Actor%20Object%20Reference)))

(event EventTick
  (params (DeltaSeconds :type Float%20%28single-precision%29)))

(fn ConstructionScript)