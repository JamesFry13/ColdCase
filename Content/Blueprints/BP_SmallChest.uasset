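; Small chest actor whose drawers slide open and closed, with a sound, when its SmallDrawerInteract event fires.
; A line trace from the first-person camera picks the static mesh drawer, and its relative Y position decides whether to open or close.
; Two timelines lerp that mesh along local Y by a fixed offset.
; CanOpen blocks re-entry during movement, but stays false if a cast fails.
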(event EventBeginPlay
  (Input|EnableInput (Game|GetPlayerController 0) 0))

(event EventSmallDrawerInteract
  (bind _returnvalue (Transformation|GetActorLocation))
  ;[0.3708 1 0.3656] Main Functionality
  (if (Variables|Default|GetCan%20Open)
    (Variables|Default|SetCan%20Open false)
    (bind _asbp_first_person_character (Utilities|Casting|CastToBP_FirstPersonCharacter (Game|GetPlayerCharacter 0)))
    (bind (_outhit _returnvalue_2) (Collision|LineTraceForObjects (Transformation|GetWorldLocation (Variables|/Game/Blueprints/BP_FirstPersonCharacter.BP_FirstPersonCharacter_C|GetFirstPersonCamera _asbp_first_person_character)) (+ (Transformation|GetWorldLocation (Variables|/Game/Blueprints/BP_FirstPersonCharacter.BP_FirstPersonCharacter_C|GetFirstPersonCamera _asbp_first_person_character)) (* (Math|Vector|GetForwardVector (Variables|/Game/Blueprints/BP_FirstPersonCharacter.BP_FirstPersonCharacter_C|GetFirstPersonCamera _asbp_first_person_character)) (Math|Vector|MakeVector 5e+02 5e+02 5e+02))) (Utilities|Array|MakeArray "ObjectTypeQuery2") false 0 "ForDuration" false))
    (if _returnvalue_2
      (bind _asstatic_mesh_component (Utilities|Casting|CastToStaticMeshComponent (.HitComponent (Collision|BreakHitResult _outhit)))
        (:then
          (Variables|Default|SetAs%20Static%20Mesh%20Component _asstatic_mesh_component)
          (if (not (>= (.y (Variables|/Script/Engine.SceneComponent|GetRelativeLocation _asstatic_mesh_component)) 45.0))
            (Audio|PlaySoundatLocation "/Game/Sounds/UPDATE/ES_Hotel_Room_Drawer_1_-_SFX_Producer.ES_Hotel_Room_Drawer_1_-_SFX_Producer" _returnvalue "0, 0, 0" 1.0 1.0 0.6 0 0 0 0)
            (Variables|Default|SetStart%20Loc (Math|Vector|MakeVector (.x (Variables|/Script/Engine.SceneComponent|GetRelativeLocation (Variables|Default|GetAs%20Static%20Mesh%20Component))) (.y (Variables|/Script/Engine.SceneComponent|GetRelativeLocation (Variables|Default|GetAs%20Static%20Mesh%20Component))) (.z (Variables|/Script/Engine.SceneComponent|GetRelativeLocation (Variables|Default|GetAs%20Static%20Mesh%20Component)))))
            (Variables|Default|SetEnd%20Loc (Math|Vector|MakeVector (.x (Variables|/Script/Engine.SceneComponent|GetRelativeLocation (Variables|Default|GetAs%20Static%20Mesh%20Component))) (+ (.y (Variables|/Script/Engine.SceneComponent|GetRelativeLocation (Variables|Default|GetAs%20Static%20Mesh%20Component))) 45.0) (.z (Variables|/Script/Engine.SceneComponent|GetRelativeLocation (Variables|Default|GetAs%20Static%20Mesh%20Component)))))
            (bind _open (Timeline|Timeline PlayFromStart)
              (:Update
                (Transformation|SetRelativeLocation (Variables|Default|GetAs%20Static%20Mesh%20Component) (Math|Vector|Lerp(Vector) (Variables|Default|GetStart%20Loc) (Variables|Default|GetEnd%20Loc) _open) false false))
              (:Finished
                (Variables|Default|SetCan%20Open true)))
            (else
              (Audio|PlaySoundatLocation "/Game/Sounds/UPDATE/ES_Drawer_Close_Hotel_4_-_SFX_Producer.ES_Drawer_Close_Hotel_4_-_SFX_Producer" _returnvalue "0, 0, 0" 1.0 1.0 0.2 0 0 0 0)
              ;[1 0 0] Close
              (Variables|Default|SetStart%20Loc (Math|Vector|MakeVector (.x (Variables|/Script/Engine.SceneComponent|GetRelativeLocation (Variables|Default|GetAs%20Static%20Mesh%20Component))) (.y (Variables|/Script/Engine.SceneComponent|GetRelativeLocation (Variables|Default|GetAs%20Static%20Mesh%20Component))) (.z (Variables|/Script/Engine.SceneComponent|GetRelativeLocation (Variables|Default|GetAs%20Static%20Mesh%20Component)))))
              (Variables|Default|SetEnd%20Loc (Math|Vector|MakeVector (.x (Variables|/Script/Engine.SceneComponent|GetRelativeLocation (Variables|Default|GetAs%20Static%20Mesh%20Component))) (- (.y (Variables|/Script/Engine.SceneComponent|GetRelativeLocation (Variables|Default|GetAs%20Static%20Mesh%20Component))) 45.0) (.z (Variables|/Script/Engine.SceneComponent|GetRelativeLocation (Variables|Default|GetAs%20Static%20Mesh%20Component)))))
              (bind _open_2 (Timeline|Timeline_0 PlayFromStart)
                (:Update
                  (Transformation|SetRelativeLocation (Variables|Default|GetAs%20Static%20Mesh%20Component) (Math|Vector|Lerp(Vector) (Variables|Default|GetStart%20Loc) (Variables|Default|GetEnd%20Loc) _open_2) false false))
                (:Finished
                  (Variables|Default|SetCan%20Open true))))))
        (:CastFailed
          (Development|PrintString "Hello")))
      (else
        (Variables|Default|SetCan%20Open true)))))

(fn ConstructionScript)