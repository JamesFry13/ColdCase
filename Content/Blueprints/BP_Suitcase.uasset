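; BP_Suitcase is an interactable suitcase with a lockbox lid that swings open and shut.
; A sphere overlap creates an interact prompt widget on screen, removed on end overlap, without filtering the overlapping actor.
; The Open/CloseLockbox event, not invoked within this graph, uses a FlipFlop to play or reverse a timeline that pitches the lid, with a sound for each direction.
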(event OnComponentBeginOverlap(Sphere)
  (params (OverlappedComponent :type Primitive%20Component%20Object%20Reference) (OtherActor :type Actor%20Object%20Reference) (OtherComp :type Primitive%20Component%20Object%20Reference) (OtherBodyIndex :type Integer) (bFromSweep :type Boolean) (SweepResult :type Hit%20Result%20Structure%20%28by%20ref%29))
  (bind _returnvalue (UserInterface|CreateWidget "/Game/Widgets/WBP_InteractPrompt.WBP_InteractPrompt_C"))
  (UserInterface|Viewport|AddtoViewport _returnvalue 0))

(event OnComponentEndOverlap(Sphere)
  (params (OverlappedComponent :type Primitive%20Component%20Object%20Reference) (OtherActor :type Actor%20Object%20Reference) (OtherComp :type Primitive%20Component%20Object%20Reference) (OtherBodyIndex :type Integer))
  (Widget|RemovefromParent (stale OnComponentBeginOverlap(Sphere) _returnvalue)))

(event Custom|Open/Close%20Lockbox
  (bind _lock_box_lid (Variables|Default|GetLock_Box_Lid))
  (bind _returnvalue (Transformation|GetWorldLocation _lock_box_lid))
  ;[1 0.442 0.09453] Open/Close
  (Utilities|FlowControl|FlipFlop
    (:A
      (Audio|PlaySoundatLocation "/Engine/VREditor/Sounds/UI/Scaling_Up.Scaling_Up" _returnvalue "0, 0, 0" 1.0 1.0 0.0 0 0 0 0)
      (bind _doorfloat (Timeline|Timeline Play)
        (:Update
          (Transformation|SetRelativeRotation (Variables|Default|GetLock_Box_Lid) (Math|Rotator|MakeRotator 0.0 (Math|Float|Lerp 0.0 -1.2e+02 _doorfloat) 0.0) false false))))
    (:B
      (Audio|PlaySoundatLocation "/Engine/VREditor/Sounds/UI/Scaling_Down.Scaling_Down" _returnvalue "0, 0, 0" 1.0 1.0 0.0 0 0 0 0)
      (Timeline|Timeline Reverse))))

(event EventBeginPlay)

(event Collision|EventActorBeginOverlap
  (params (OtherActor :type Actor%20Object%20Reference)))

(event EventTick
  (params (DeltaSeconds :type Float%20%28single-precision%29)))

(fn ConstructionScript)