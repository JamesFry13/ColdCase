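; Blueprint for a single chest of drawers with one drawer that slides open and closed.
; The Drawer_1 event uses a FlipFlop to alternately play and reverse a timeline that lerps the drawer's relative Y position, playing a cupboard door sound at the drawer each time.
; The Interact input only casts to the first-person character and triggers nothing further, and nothing in this graph calls Drawer_1.
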(event Custom|Drawer_1
  (bind _drawer1 (Variables|Default|GetDrawer1))
  (bind _returnvalue (Transformation|GetWorldLocation _drawer1))
  ;[0.205 1 0.7148] Open Draw 1
  (Utilities|FlowControl|FlipFlop
    (:A
      (Audio|PlaySoundatLocation "/Game/Sounds/raw/cupboarddoor.cupboarddoor" _returnvalue "0, 0, 0" 1.0 1.0 0.0 0 0 0 0)
      (bind _doorfloat (Timeline|Timeline Play)
        (:Update
          (Transformation|SetRelativeLocationAndRotation (Variables|Default|GetDrawer1) (Math|Vector|MakeVector 0.0 (Math|Float|Lerp 0.0 -5e+01 _doorfloat) 0.0) "0, 0, 0" false false))))
    (:B
      (Audio|PlaySoundatLocation "/Game/Sounds/raw/cupboarddoor.cupboarddoor" _returnvalue "0, 0, 0" 1.0 1.0 0.0 0 0 0 0)
      (Timeline|Timeline Reverse))))

(event Input|ActionEvents|InputActionInteract
  (params (Key :type Key%20Structure :default "None"))
  (:Pressed
    (Utilities|Casting|CastToBP_FirstPersonCharacter (Game|GetPlayerCharacter 0))))

(fn ConstructionScript)